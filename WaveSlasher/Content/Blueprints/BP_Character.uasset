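; Player character Blueprint that handles camera look, movement and a three-swing sword attack.
; Enhanced Input drives controller yaw/pitch and yaw-relative movement.
; Attack input, blocked while attacking, plays the montage selected by AttackCount on the Sword mesh, incrementing the count after a retriggerable delay.
; Montage completion resets attack state and count immediately; interruption resets them after a delay.
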(event Input|EnhancedActionEvents|EnhancedInputActionIA_Look
  (params (ActionValue :type Vector%202D%20Structure) (ElapsedSeconds :type Float%20%28double-precision%29) (TriggeredSeconds :type Float%20%28double-precision%29) (InputAction :type Input%20Action%20Object%20Reference :default "/Game/Inputs/IA_Look.IA_Look"))
  (Pawn|Input|AddControllerYawInput (.x ActionValue))
  (Pawn|Input|AddControllerPitchInput (.y ActionValue)))

(event Input|EnhancedActionEvents|EnhancedInputActionIA_MoveFB
  (params (ActionValue :type Float%20%28double-precision%29) (ElapsedSeconds :type Float%20%28double-precision%29) (TriggeredSeconds :type Float%20%28double-precision%29) (InputAction :type Input%20Action%20Object%20Reference :default "/Game/Inputs/IA_MoveFB.IA_MoveFB"))
  (Pawn|Input|AddMovementInput (Math|Vector|GetForwardVector (Math|Rotator|MakeRotator 0.0 0.0 (.yaw (Pawn|GetControlRotation :!class /Script/Engine.Pawn)))) ActionValue false))

(event Input|EnhancedActionEvents|EnhancedInputActionIA_MoveRL
  (params (ActionValue :type Float%20%28double-precision%29) (ElapsedSeconds :type Float%20%28double-precision%29) (TriggeredSeconds :type Float%20%28double-precision%29) (InputAction :type Input%20Action%20Object%20Reference :default "/Game/Inputs/IA_MoveRL.IA_MoveRL"))
  (Pawn|Input|AddMovementInput (Math|Vector|GetRightVector (Math|Rotator|MakeRotator 0.0 0.0 (.yaw (Pawn|GetControlRotation :!class /Script/Engine.Pawn)))) ActionValue false))

(event Input|ActionEvents|InputActionAttack
  (params (Key :type Key%20Structure :default "None"))
  (:Pressed
    (if (not (Variables|Default|GetCharacterAttacking))
      (Animation|Montage|PlayMontage (Variables|Default|GetSword) (Utilities|Select :Index (Variables|Default|GetAttackCount) :Option%200 "/Game/ArtAnim/Animations/Pardis3SwordRLSwing_Montage.Pardis3SwordRLSwing_Montage" :Option%201 "/Game/ArtAnim/Animations/Pardis3SwordSwingLR1_Montage.Pardis3SwordSwingLR1_Montage" :Option%202 "/Game/ArtAnim/Animations/Pardis3SwordSwingUD_Montage.Pardis3SwordSwingUD_Montage")
        (:then
          (Variables|Default|SetCharacterAttacking true)
          (Utilities|FlowControl|RetriggerableDelay 1.0)
          (Math|Integer|IncrementInt (Variables|Default|GetAttackCount)))
        (:OnCompleted
          (Variables|Default|SetCharacterAttacking false)
          (Variables|Default|SetAttackCount 0 :!label _label))
        (:OnInterrupted
          (Utilities|FlowControl|RetriggerableDelay 1.5)
          (Variables|Default|SetCharacterAttacking false)
          (goto _label))))))

(fn ConstructionScript)